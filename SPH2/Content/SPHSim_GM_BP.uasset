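; SPH fluid simulation manager, likely a Game Mode, that spawns a block of Particle_BP actors inside a box of point-normal planes.
; BeginPlay sets up planes, fluid constants, grid and particles.
; Each Tick rebuilds the grid, computes densities and forces, then resolves plane collisions and integrates particles at a fixed timestep.
; A sine offset shifts one wall as a wave maker and moves all StaticMeshActors, as the "plane" tag check filters nothing.
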(event `InputAction|MovePlaneLeft`
  (params (Key :type "Key Structure")))

(event `InputAction|MovePlaneRight`
  (params (Key :type "Key Structure")))

(event `self.ReceiveBeginPlay`
  (`self.PlacePlanes`)
  (`self.InitializeConstants`)
  (`self.InitializeParticles`)
  (`self.EnableInput` (`GameplayStatics.GetPlayerController` 0)))

(event `self.ReceiveTick`
  (params (DeltaSeconds :type "Float (single-precision)"))
  (bind _returnvalue (+ (`self.Ftime`) 0.02))
  (bind _returnvalue_2 (* (`KismetMathLibrary.MakeVector` 0.0 (`KismetMathLibrary.Sin` _returnvalue)) -1.0))
  (bind _outactors (`GameplayStatics.GetAllActorsOfClass` "/Game/Particle_BP.Particle_BP_C"))
  (if (!= (`KismetArrayLibrary.Array_Length` _outactors) 0)
    (`self.ConstructGrid` 1000)
    (`self.ComputeDensities`)
    (`self.ComputeForces`)
    (for (_array_element _array_index) _outactors
      (`self.popParticleFromGrid` _array_index)
      (`self.CheckParticlePlanesCollision` _array_element)
      (`Particle.Update` _array_element 0.01)
      (`/Game/Particle_BP.UpdateWorldLocation` _array_element))
    (bind _outactors_2 (`GameplayStatics.GetAllActorsOfClass` "/Script/Engine.StaticMeshActor"))
    (for _array_element_2 _outactors_2
      (if (`self.ActorHasTag` _array_element_2 "plane")
        _
        (else
          _))
      (set `self.Ftime` _returnvalue)
      (`self.K2_SetActorLocation` _array_element_2 (+ (`self.K2_GetActorLocation` _array_element_2) _returnvalue_2) false false))
    (`self.SetPlaneRight` (+ (`|GetArrayItem` (`self.planes`) 6) _returnvalue_2))))

(fn `InitializeConstants`
  (set `self.gravity` (0.0 0.0 -9.81))
  (set `self.mass` 0.02)
  (set `self.visc_coeff` 3.0)
  (set `self.tension_coeff` 0.1028)
  (set `self.rest_density` 998.289978)
  (set `self.Kp` 3.0)
  (`self.setH` 0.0457)
  (set `self.gridDimension` (50.0 100.0 200.0))
  (set `self.simOffset` (0.0 100.0 50.0))
  (`self.setGrid`))

(fn `InitializeParticles`
  (locals (dimX :type Integer :default 0) (dimY :type Integer) (dimZ :type Integer) (spaceBetween :type "Float (double-precision)" :default 4.0))
  (bind _dimy (`local.dimY`))
  (while (< (`local.dimX`) 10)
    (while (< _dimy 10)
      (while (< (`local.dimZ`) 20)
        (if (== _dimy 0)
          _
          (else
            _))
        (`self.SpawnNewParticle` (+ (* (`KismetMathLibrary.MakeVector` (`KismetMathLibrary.Conv_IntToDouble` (`local.dimX`)) (`KismetMathLibrary.Conv_IntToDouble` (`local.dimY`)) (`KismetMathLibrary.Conv_IntToDouble` (`local.dimZ`))) (`local.spaceBetween`)) (30.0 -45.0 5.0)) (0.0 0.0 0.0) (`self.gravity`))
        (set `local.dimZ` (+ (`local.dimZ`) 1)))
      (set `local.dimY` (+ (`local.dimY`) 1))
      (set `local.dimZ` 0))
    (set `local.dimX` (+ (`local.dimX`) 1))
    (set `local.dimY` 0))
  (return))

(fn `PlacePlanes`
  (bind _planes (`self.planes`))
  (`KismetArrayLibrary.Array_Clear` _planes)
  (`KismetArrayLibrary.Array_Add` _planes)
  (`KismetArrayLibrary.Array_Add` _planes (0.0 0.0 1.0))
  (`KismetArrayLibrary.Array_Add` _planes (75.0 0.0 0.0))
  (`KismetArrayLibrary.Array_Add` _planes (-1.0 0.0 0.0))
  (`KismetArrayLibrary.Array_Add` _planes (25.0 0.0 0.0))
  (`KismetArrayLibrary.Array_Add` _planes (1.0 0.0 0.0))
  (`KismetArrayLibrary.Array_Add` _planes (0.0 50.0 0.0))
  (`KismetArrayLibrary.Array_Add` _planes (0.0 -1.0 0.0))
  (`KismetArrayLibrary.Array_Add` _planes (0.0 -50.0 0.0))
  (`KismetArrayLibrary.Array_Add` _planes (0.0 1.0 0.0)))

(fn `SetPlaneRight`
  (params (AddPos :type "Vector Structure"))
  (bind _planes (`self.planes`))
  (`KismetArrayLibrary.Array_Clear` _planes)
  (`KismetArrayLibrary.Array_Add` _planes)
  (`KismetArrayLibrary.Array_Add` _planes (0.0 0.0 1.0))
  (`KismetArrayLibrary.Array_Add` _planes (75.0 0.0 0.0))
  (`KismetArrayLibrary.Array_Add` _planes (-1.0 0.0 0.0))
  (`KismetArrayLibrary.Array_Add` _planes (25.0 0.0 0.0))
  (`KismetArrayLibrary.Array_Add` _planes (1.0 0.0 0.0))
  (`KismetArrayLibrary.Array_Add` _planes AddPos)
  (`KismetArrayLibrary.Array_Add` _planes (0.0 -1.0 0.0))
  (`KismetArrayLibrary.Array_Add` _planes (0.0 -50.0 0.0))
  (`KismetArrayLibrary.Array_Add` _planes (0.0 1.0 0.0)))

(fn `SpawnNewParticle`
  (params (Position :type "Vector Structure") (Velocity :type "Vector Structure") (Acceleration :type "Vector Structure"))
  (bind _returnvalue (`|SpawnActorFromClass` "/Game/Particle_BP.Particle_BP_C" (`KismetMathLibrary.MakeTransform` Position) "Undefined" "OverrideRootScale" null null))
  (`KismetArrayLibrary.Array_Add` (`self.particles`) _returnvalue)
  (set `Particle.velocity` Velocity _returnvalue)
  (set `Particle.acceleration` Acceleration _returnvalue)
  (bind _output_get (set `Particle.position` Position _returnvalue))
  (set `Particle.prevPosition` _output_get _returnvalue))

(fn `UserConstructionScript`)