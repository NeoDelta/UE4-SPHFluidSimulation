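; Controller Blueprint with no active logic: its BeginPlay and Tick events are disabled placeholders and its construction script is empty.
; Disconnected graph fragments appear to experiment with nudging a position along the Y axis in opposite directions, through a Planes vector array or by moving a StaticMeshActor found with GetAllActorsOfClass.
; None of these fragments can run, including a debug "Hello" print.
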(event `InputAction|MovePlaneLeft`
  (params (Key :type "Key Structure")))

(event `InputAction|MovePlaneRight`
  (params (Key :type "Key Structure")))

(fn `UserConstructionScript`)